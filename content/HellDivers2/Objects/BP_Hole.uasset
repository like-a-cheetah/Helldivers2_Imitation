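; BP_Hole is a hole object with a Stat component that shuts down its smoke and light when HP reaches zero.
; On BeginPlay it binds to the Stat component's HP-zero event, which deactivates the smoke particle and starts a looping timer.
; Each timer tick dims the point light by a delta-time-scaled step, then destroys it and clears the timer as intensity runs out.
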(event `self.ReceiveBeginPlay`
  (add `CharacterStatComponent.OnHpZero` (`self.Stat`) (delegate `OnHpZero_이벤트`)))

(event `OnHpZero_이벤트`
  (`ActorComponent.SetActive` (`self.P_Smoke_B1`) false false)
  (`KismetSystemLibrary.K2_SetTimerDelegate` (delegate `FadeOutLight`) 0.1 true))

(event `FadeOutLight`
  (bind _returnvalue (- (`LightComponentBase.Intensity` (`self.PointLight`)) (* (`GameplayStatics.GetWorldDeltaSeconds`) 100000.0)))
  (`LightComponent.SetIntensity` (`self.PointLight`) _returnvalue)
  (if (<= _returnvalue 0.0)
    (`ActorComponent.K2_DestroyComponent` (`self.PointLight`))
    (`KismetSystemLibrary.K2_ClearTimer` null "FadeOutLight")))

(fn `UserConstructionScript`)