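; Resupply stratagem hellpod attachment that carries ammo boxes and folds the pod away once all of them are gone.
; On BeginPlay it destroys its trigger collision, then spawns an ammo box for each socket name and attaches it there.
; Each box's OnDestroyed event removes it from the tracked array, and an empty array calls FoldHellpod.
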(event `self.ReceiveBeginPlay`
  (`ActorComponent.K2_DestroyComponent` (`self.TiggerCollision`))
  (for _array_element (`self.AmmoBoxeSockets`)
    (bind _returnvalue (`|SpawnActorFromClass` "/Game/HellDivers2/Items/BP_AmmoBox.BP_AmmoBox_C" (`SceneComponent.K2_GetComponentToWorld` (`self.SkelMeshComp`)) "AlwaysSpawn" "MultiplyWithRoot" self null))
    (`KismetArrayLibrary.Array_Add` (`self.Boxes`) _returnvalue)
    (add `self.OnDestroyed` _returnvalue (delegate `커스텀이벤트`))
    (`self.K2_AttachToActor` _returnvalue self _array_element "SnapToTarget" "SnapToTarget" "KeepWorld" false)))

(event `커스텀이벤트` :!signature `self.OnDestroyed`
  (params (DestroyedActor :type "Actor Object Reference"))
  (bind _boxes (`self.Boxes`))
  (`KismetArrayLibrary.Array_RemoveItem` _boxes DestroyedActor)
  (if (not (`KismetMathLibrary.Conv_IntToBool` (`KismetArrayLibrary.Array_Length` _boxes)))
    (`self.FoldHellpod`)))

(fn `UserConstructionScript`)