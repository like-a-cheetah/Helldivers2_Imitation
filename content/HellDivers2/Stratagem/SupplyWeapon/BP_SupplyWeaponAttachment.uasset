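; Weapon supply hellpod attachment for a HellDivers 2-style stratagem, carrying a gun until it is detached.
; On BeginPlay it destroys its trigger collision, spawns the configured gun class and snaps it to the attach0 socket.
; It binds to the gun's detach-from-hellpod dispatcher, then folds the hellpod and unbinds when that fires.
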(event `self.ReceiveBeginPlay`
  (`ActorComponent.K2_DestroyComponent` (`self.TiggerCollision`))
  (bind _returnvalue (`|SpawnActorFromClass` (`self.GunC`) (`self.GetTransform` self) "AlwaysSpawn" "MultiplyWithRoot" self))
  (add `Gun.OnDetachFromSupplyHellpod` _returnvalue (delegate `OnDetachFromSupplyHellpod_이벤트`))
  (`self.K2_AttachToActor` _returnvalue self "attach0" "SnapToTarget" "SnapToTarget" "KeepRelative" false))

(event `OnDetachFromSupplyHellpod_이벤트`
  (`self.FoldHellpod`)
  (remove `Item.OnDetachFromSupplyHellpod` (stale `self.ReceiveBeginPlay` _returnvalue) (delegate `OnDetachFromSupplyHellpod_이벤트`)))

(fn `UserConstructionScript`)